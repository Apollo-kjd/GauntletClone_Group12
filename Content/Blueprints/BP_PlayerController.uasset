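; Player controller that caches the player pawn on BeginPlay and turns input into movement data and character actions.
; Vertical and horizontal axis events share one step that stores a MoveVector, and vertical input also sets an UpDirFix flag at full positive value.
; Shoot and UsePotion presses cast the cached pawn to BP_Character and call the matching function.
; The movement values are only stored here, not applied to the pawn.
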(event EventBeginPlay
  ;[0 0 0] Get Ref to Player Pawn
  (Variables|Default|SetPlayerPawnRef (Game|Player|GetPlayerPawn 0)))

(event Input|ActionEvents|InputActionShoot
  (params (Key :type Key%20Structure :default "None"))
  ;[0 0 0] Get Input
  (:Pressed
    (bind _asbp_character (Utilities|Casting|CastToBP_Character (Variables|Default|GetPlayerPawnRef)))
    (Default|Shoot _asbp_character)))

(event Input|ActionEvents|InputActionUsePotion
  (params (Key :type Key%20Structure :default "None"))
  ;[0 0 0] Get Input
  (:Pressed
    (bind _asbp_character (Utilities|Casting|CastToBP_Character (Variables|Default|GetPlayerPawnRef)))
    (Default|UsePotion _asbp_character)))

(event Input|AxisEvents|InputAxisHorzInput
  (params (AxisValue :type Float%20%28single-precision%29))
  ;[0 0 0] Get Input
  (Variables|Default|SetMoveVector (Math|Vector|MakeVector (stale Input|AxisEvents|InputAxisVertInput AxisValue) AxisValue 0.0)))

(event Input|AxisEvents|InputAxisVertInput
  (params (AxisValue :type Float%20%28single-precision%29))
  ;[0 0 0] Get Input
  (Variables|Default|SetUpDirFix (== AxisValue 1.0))
  (Variables|Default|SetMoveVector (Math|Vector|MakeVector AxisValue (stale Input|AxisEvents|InputAxisHorzInput AxisValue) 0.0)))

(fn ConstructionScript)