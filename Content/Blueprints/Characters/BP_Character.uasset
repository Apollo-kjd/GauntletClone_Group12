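; Player character that moves, shoots, deals melee damage on overlap, and loses health each second and when damaged, opening a level at zero.
; Tick applies a swept offset from the BP_PlayerController's MoveVector and rotates to face it, using UpDirFix to allow the otherwise skipped zero rotation.
; Shoot spawns BP_Projectile at the Sphere component's transform.
; UsePotion is an empty stub.
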(event Custom|HealthTimer
  ;[0 0 0] Cast to Controller and Tick Health
  (Math|Float|DecrementFloat (Variables|Default|GetHealth)
    (:%20%20
      (if (<= (Variables|Default|GetHealth) 0.0)
        (Game|OpenLevel(byObjectReference))))))

(event Custom|Shoot
  ;[0 0 0] Shoot
  (Game|SpawnActorfromClass "/Game/Blueprints/BP_Projectile.BP_Projectile_C" (Transformation|GetWorldTransform (Variables|Default|GetSphere)) "Undefined" 0 0))

(event Custom|UsePotion)

(event EventBeginPlay
  ;[0 0 0] Cast to Controller and Tick Health
  (bind _asbp_player_controller (Utilities|Casting|CastToBP_PlayerController (Game|GetPlayerController 0)))
  (Variables|Default|SetPlayerController _asbp_player_controller)
  (Utilities|Time|SetTimerbyEvent (delegate Custom|HealthTimer) 1.0 true))

(event EventTick
  (params (DeltaSeconds :type Float%20%28single-precision%29))
  (bind _playercontroller (Variables|Default|GetPlayerController))
  (bind _movevector (Variables|/Game/Blueprints/BP_PlayerController.BP_PlayerController_C|GetMoveVector _playercontroller))
  (bind _returnvalue (Math|Conversions|RotationFromXVector _movevector))
  ;[0 0 0] Move
  (Transformation|AddActorWorldOffset (* DeltaSeconds (Variables|Default|GetMoveSpeed) _movevector (Variables|Default|GetRunSpeed)) true)
  (if (Utilities|Operators|EqualEqual :A _returnvalue)
    (if (Variables|/Game/Blueprints/BP_PlayerController.BP_PlayerController_C|GetUpDirFix (Variables|Default|GetPlayerController))
      (Transformation|SetActorRotation _returnvalue :!label _label))
    (else
      (goto _label))))

(event Game|Damage|EventAnyDamage
  (params (Damage :type Float%20%28single-precision%29) (DamageType :type Damage%20Type%20Object%20Reference) (InstigatedBy :type Controller%20Object%20Reference) (DamageCauser :type Actor%20Object%20Reference))
  ;[0 0 0] Cast to Controller and Tick Health
  (Variables|Default|SetHealth (- (Variables|Default|GetHealth) Damage))
  (if (<= (Variables|Default|GetHealth) 0.0)
    (Game|OpenLevel(byObjectReference))))

(event Collision|EventActorBeginOverlap
  (params (OtherActor :type Actor%20Object%20Reference))
  ;[0 0 0] Melee
  (Game|Damage|ApplyDamage OtherActor (Math|Conversions|ToFloat(Integer) (Variables|Default|GetMeleeDamage)) 0 0))

(fn ConstructionScript)